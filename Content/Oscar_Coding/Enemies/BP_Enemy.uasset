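; BP_Enemy is an enemy actor that homes in on the player and knocks them away on contact.
; It caches the first BP_Player at BeginPlay.
; Any overlap with the TargetPLayer component switches its ProjectileMovement to strong homing on the player's root component.
; Any overlap with Sphere launches the cached player along the enemy's forward vector scaled by LaunchForce, with a fixed upward boost; ApplyStats is an empty stub.
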(event OnComponentBeginOverlap(Sphere)
  (params (OverlappedComponent :type Primitive%20Component%20Object%20Reference) (OtherActor :type Actor%20Object%20Reference) (OtherComp :type Primitive%20Component%20Object%20Reference) (OtherBodyIndex :type Integer) (bFromSweep :type Boolean) (SweepResult :type Hit%20Result%20Structure%20%28by%20ref%29))
  (bind _returnvalue (Transformation|GetActorForwardVector))
  (bind _launchforce (Variables|Default|GetLaunchForce))
  (bind _returnvalue_2 (* _returnvalue _launchforce))
  (bind _player (Variables|Default|GetPlayer)
    (:then
      (Character|LaunchCharacter _player (Math|Vector|MakeVector (.x _returnvalue_2) (.y _returnvalue_2) 1e+03) false false))
    (:else)))

(event OnComponentBeginOverlap(TargetPLayer)
  (params (OverlappedComponent :type Primitive%20Component%20Object%20Reference) (OtherActor :type Actor%20Object%20Reference) (OtherComp :type Primitive%20Component%20Object%20Reference) (OtherBodyIndex :type Integer) (bFromSweep :type Boolean) (SweepResult :type Hit%20Result%20Structure%20%28by%20ref%29))
  (CallFunction|HomeonPlayer (Variables|Default|GetPlayer)))

(event Custom|Home%20on%20Player
  (params (Target :type BP%20Player%20Object%20Reference))
  (bind _projectilemovement (Variables|Default|GetProjectileMovement))
  (Variables|/Script/Engine.ProjectileMovementComponent|SetHomingTargetComponent _projectilemovement (Variables|/Script/Engine.Actor|GetRootComponent Target))
  (Variables|/Script/Engine.ProjectileMovementComponent|SetbIsHomingProjectile _projectilemovement true)
  (Variables|/Script/Engine.ProjectileMovementComponent|SetHomingAccelerationMagnitude _projectilemovement 4e+04))

(event EventBeginPlay
  (bind _returnvalue (Actor|GetActorOfClass "/Game/Oscar_Coding/oscar_Blueprints/BP_Player.BP_Player_C"))
  (Variables|Default|SetPlayer _returnvalue))

(fn ConstructionScript)

(fn ApplyStats
  (return ""))