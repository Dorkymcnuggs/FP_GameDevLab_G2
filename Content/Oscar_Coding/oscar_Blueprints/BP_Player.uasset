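; First-person player character Blueprint with sprinting, wall running, wall jumps, zipline entry, pickup boosts and an inventory bar.
; A looping timer, started by jumping while sprinting, line-traces both sides, lowers gravity and launches the player along the wall, while Tick tilts the camera.
; Items load from the game instance into a scroll-selected widget bar for consuming or dropping.
; Speed and jump boosts scale movement values.
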(event OnComponentBeginOverlap(CapsuleComponent)
  (params (OverlappedComponent :type Primitive%20Component%20Object%20Reference) (OtherActor :type Actor%20Object%20Reference) (OtherComp :type Primitive%20Component%20Object%20Reference) (OtherBodyIndex :type Integer) (bFromSweep :type Boolean) (SweepResult :type Hit%20Result%20Structure%20%28by%20ref%29))
  ;[0.15 0.15 0.15 0.5] Checks Pickups
  (Class|BPIDelivery|ApplyStats(Message) OtherActor)
  (Utilities|Platform|CollectGarbage))

(event Custom|Stop%20Wall%20Run%20Timer
  ;[0.15 0.15 0.15 0.5] Wall Run timer also checks for walls
  (Utilities|Time|ClearandInvalidateTimerbyHandle (Variables|WallRunning|GetWallRunTimer))
  (WallRun|ApplyWallRunVariable 1.0 false false false))

(event Custom|Start%20Wall%20Run%20Timer
  ;[0.15 0.15 0.15 0.5] Wall Run timer also checks for walls
  (bind _returnvalue (Utilities|Time|SetTimerbyEvent (delegate Custom|Wall%20Check) 0.001 true false 0.2))
  (Variables|WallRunning|SetWallRunTimer _returnvalue))

(event Custom|Wall%20Check
  ;[0.15 0.15 0.15 0.5] Wall Run timer also checks for walls
  (WallRun|WallRunCheckWalls))

(event Input|EnhancedActionEvents|EnhancedInputActionIA_Consume
  (params (ActionValue :type Boolean) (ElapsedSeconds :type Float%20%28double-precision%29) (TriggeredSeconds :type Float%20%28double-precision%29) (InputAction :type Input%20Action%20Object%20Reference :default "/Game/Oscar_Coding/oscar_Inputs/IA_Consume.IA_Consume"))
  (bind _inventoryslot (Variables|Default|GetInventorySlot))
  (bind _items (Variables|Default|GetItems))
  (bind _inventoryslot_2 (Variables|Default|GetInventorySlot))
  (bind _output (Utilities|Array|Get(acopy) _items _inventoryslot_2))
  (bind (_itemclass _itemtype) (Utilities|Struct|BreakS_ItemInfo _output))
  ;[0.15 0.15 0.15 0.5] Checks Pickups
  (:Completed
    (if (Utilities|Enum|Equal(Enum) _itemtype "NewEnumerator1")
      (bind _returnvalue (Game|SpawnActorfromClass _itemclass (Math|Transform|MakeTransform "0, 0, 0") "Undefined" "MultiplyWithRoot" 0 0))
      (switch Utilities|FlowControl|Switch|SwitchonEN_ItemType _itemtype
        (:NewEnumerator1
          (Class|BPIDelivery|ActivateConsume(Message) _returnvalue)
          (Utilities|Array|SetArrayElem (Variables|Default|GetItems) _inventoryslot (Utilities|Struct|MakeS_ItemInfo "None" "/Game/Oscar_Coding/oscar_Materials/T_EmptySlotCon.T_EmptySlotCon" true 0 "NewEnumerator3" 0))
          (Class|BPIDelivery|SetIcon(Message) (Variables|Default|GetIWidget) _inventoryslot "/Game/Oscar_Coding/oscar_Materials/T_EmptySlotCon.T_EmptySlotCon"))))))

(event Input|EnhancedActionEvents|EnhancedInputActionIA_FBMove
  (params (ActionValue :type Float%20%28double-precision%29) (ElapsedSeconds :type Float%20%28double-precision%29) (TriggeredSeconds :type Float%20%28double-precision%29) (InputAction :type Input%20Action%20Object%20Reference :default "/Game/Oscar_Coding/oscar_Inputs/IA_FBMove.IA_FBMove"))
  ;[0.15 0.15 0.15 0.5] Move left and Right, Forward and Back
  (Pawn|Input|AddMovementInput (Transformation|GetActorForwardVector) ActionValue false))

(event Input|EnhancedActionEvents|EnhancedInputActionIA_LRMove
  (params (ActionValue :type Float%20%28double-precision%29) (ElapsedSeconds :type Float%20%28double-precision%29) (TriggeredSeconds :type Float%20%28double-precision%29) (InputAction :type Input%20Action%20Object%20Reference :default "/Game/Oscar_Coding/oscar_Inputs/IA_LRMove.IA_LRMove"))
  ;[0.15 0.15 0.15 0.5] Move left and Right, Forward and Back
  (Pawn|Input|AddMovementInput (Transformation|GetActorRightVector) ActionValue false))

(event Input|EnhancedActionEvents|EnhancedInputActionIA_Mouse
  (params (ActionValue :type Vector%202D%20Structure) (ElapsedSeconds :type Float%20%28double-precision%29) (TriggeredSeconds :type Float%20%28double-precision%29) (InputAction :type Input%20Action%20Object%20Reference :default "/Game/Oscar_Coding/oscar_Inputs/IA_Mouse.IA_Mouse"))
  ;[0.15 0.15 0.15 0.5] Jump and Camera Controls
  (Pawn|Input|AddControllerYawInput (.x ActionValue))
  (bind _result (Math|Float|NegateFloat (.y ActionValue))
    (:%20%20
      (Pawn|Input|AddControllerPitchInput _result))))

(event Input|EnhancedActionEvents|EnhancedInputActionIA_Sprint
  (params (ActionValue :type Boolean) (ElapsedSeconds :type Float%20%28double-precision%29) (TriggeredSeconds :type Float%20%28double-precision%29) (InputAction :type Input%20Action%20Object%20Reference :default "/Game/Oscar_Coding/oscar_Inputs/IA_Sprint.IA_Sprint"))
  ;[0.15 0.15 0.15 0.5] Sprint
  (:Started
    (if (Variables|Character|GetIs%20Speed%20Boost)
      (Variables|Character|SetSprinting true)
      (Variables|/Script/Engine.CharacterMovementComponent|SetMaxWalkSpeed (Variables|Character|GetCharacterMovement) (* (Variables|Character|GetSpeed%20Boost) (Variables|Character|GetMax%20Sprint%20Speed)))
      (Camera|SetFieldOfView (Variables|Default|GetFirstPersonCamera) 1.2e+02)
      (elif (Variables|Character|GetSprinting)
        (Variables|Character|SetSprinting false)
        (Variables|/Script/Engine.CharacterMovementComponent|SetMaxWalkSpeed (Variables|Character|GetCharacterMovement) (Variables|Character|GetMax%20Walk%20Speed))
        (Camera|SetFieldOfView (Variables|Default|GetFirstPersonCamera) 9e+01)
        (else
          (Variables|Character|SetSprinting true)
          (Variables|/Script/Engine.CharacterMovementComponent|SetMaxWalkSpeed (Variables|Character|GetCharacterMovement) (Variables|Character|GetMax%20Sprint%20Speed))
          (Camera|SetFieldOfView (Variables|Default|GetFirstPersonCamera) 1.1e+02))))))

(event Input|EnhancedActionEvents|EnhancedInputActionIA_Jump
  (params (ActionValue :type Boolean) (ElapsedSeconds :type Float%20%28double-precision%29) (TriggeredSeconds :type Float%20%28double-precision%29) (InputAction :type Input%20Action%20Object%20Reference :default "/Game/Oscar_Coding/oscar_Inputs/IA_Jump.IA_Jump"))
  ;[0.15 0.15 0.15 0.5] Jump and Camera Controls
  (:Triggered
    (if (Variables|ZiplineMechanic|GetNearZipline?)
      (if (Variables|ZiplineMechanic|GetCanZipline?)
        (Variables|WallRunning|SetCanWallRun false)
        (if (not (Variables|ZiplineMechanic|GetIsZiplining))
          (Variables|ZiplineMechanic|SetIsZiplining true)
          (Pawn|Components|CharacterMovement|SetMovementMode (Variables|Character|GetCharacterMovement) "MOVE_Flying" 0)
          (Transformation|SetActorRotation (Transformation|GetActorRotation (Variables|ZiplineMechanic|GetZipline%20Actor)) true)))
      (else
        (Character|Jump)
        (if (Variables|Character|GetSprinting)
          (if (Variables|WallRunning|GetCanWallRun)
            (if (Variables|WallRunning|GetWall%20Running)
              ;;[0.00773 0 0.15 0.5] Stops wall run, lets jump work
              (CallFunction|StopWallRunTimer)
              (WallRun|JumpfromWall)
              (Components|Animation|PlayAnimation (Variables|Character|GetMesh) "/Game/Characters/Mannequins/Anims/Unarmed/Jump/MM_WallJump.MM_WallJump" false)
              ;;[0.00773 0 0.15 0.5] After delay check wall run again
              (Utilities|FlowControl|Delay 0.4)
              (CallFunction|StartWallRunTimer)
              (else
                (CallFunction|StartWallRunTimer))))))))
  (:Completed
    (Character|StopJumping)))

(event EventBeginPlay
  ;[0.15 0.15 0.15 0.5] Set Up for controls and to call zipline class as reference
  (CallFunction|LoadPlayer)
  (CallFunction|GetRefs)
  (for (_array_element _array_index) (Variables|Default|GetItems)
    (Class|BPIDelivery|SetIcon(Message) (Variables|Default|GetIWidget) _array_index (.ItemIcon (Utilities|Struct|BreakS_ItemInfo _array_element)))
    (Math|Integer|IncrementInt _array_index)))

(event EventOnLanded
  (params (Hit :type Hit%20Result%20Structure%20%28by%20ref%29))
  ;[0.15 0.15 0.15 0.5] Checks if player lands
  (CallFunction|StopWallRunTimer)
  (Components|Animation|SetAnimationMode (Variables|Character|GetMesh) "AnimationBlueprint" true))

(event EventTick
  (params (DeltaSeconds :type Float%20%28single-precision%29))
  ;[0.15 0.15 0.15 0.5] Camera/Character tilt while wall running
  (WallRun|CameraTilting (Utilities|DeterminCameraTilt)))

(event EventItemSelect
  (params (Selected%20Item :type S%20Item%20Info%20Structure) (CurrSlot :type Integer))
  ;[0.15 0.15 0.15 0.5] Checks Pickups
  (CallFunction|PickItemSlot Selected%20Item CurrSlot))

(event EventApplyBoosts
  (params (IsJumpBoost :type Boolean) (JumpBoost :type Float%20%28double-precision%29) (IsSpeedBoost :type Boolean) (SpeedBoost :type Float%20%28double-precision%29))
  ;[0.15 0.15 0.15 0.5] Applies Speed/Jump Boost to player
  (Utilities|FlowControl|Sequence
    (:then_0
      (if IsJumpBoost
        (CallFunction|JumpBoostMath IsJumpBoost JumpBoost)))
    (:then_1
      (if IsSpeedBoost
        (CallFunction|SpeedBoostMath IsSpeedBoost SpeedBoost)))))

(event Input|MouseEvents|MouseWheelUp
  (params (Key :type Key%20Structure))
  ;[0.15 0.15 0.15 0.5] Hovers over item slot
  (:Pressed
    (if (not (== (Variables|Default|GetInventorySlot) (Variables|Default|GetMaxSlots)))
      (bind _result (Math|Integer|IncrementInt (Variables|Default|GetInventorySlot))
        (:%20%20
          (bind _output_get (Variables|Default|SetInventorySlot _result))
          (Class|BPIDelivery|ChangeSlot(Message) (Variables|Default|GetIWidget) _output_get))))))

(event Input|MouseEvents|MouseWheelDown
  (params (Key :type Key%20Structure))
  ;[0.15 0.15 0.15 0.5] Hovers over item slot
  (:Pressed
    (if (not (== (Variables|Default|GetInventorySlot) 0))
      (bind _result (Math|Integer|DecrementInt (Variables|Default|GetInventorySlot))
        (:%20%20
          (bind _output_get (Variables|Default|SetInventorySlot _result))
          (Class|BPIDelivery|ChangeSlot(Message) (Variables|Default|GetIWidget) _output_get))))))

(fn ConstructionScript)

(fn WallRunCheckWalls
  (bind (_start _end) (Utilities|WallChecking -1.0))
  (bind (_start_2 _end_2) (Utilities|WallChecking 1.0))
  ;[0.00773 0 0.15 0.5] Checks walls (Right)
  (bind (_outhit _returnvalue) (Collision|LineTraceForObjects _start_2 _end_2 (Utilities|Array|MakeArray "ObjectTypeQuery16") false 0 "None"))
  (if _returnvalue
    (Variables|WallRunning|SetWall%20Run%20IN (.ImpactNormal (Collision|BreakHitResult _outhit)))
    ;[0.00773 0 0.15 0.5] Checks fall speed
    (if (Utilities|FallSpeed)
      (WallRun|ApplyWRFRight -1.0)
      (else
        (WallRun|ApplyWallRunVariable 1.0 false false false :!label _label)))
    (else
      ;[0.00773 0 0.15 0.5] Checks walls (Left)
      (bind (_outhit_2 _returnvalue_2) (Collision|LineTraceForObjects _start _end (Utilities|Array|MakeArray "ObjectTypeQuery16") false 0 "None"))
      (if _returnvalue_2
        (Variables|WallRunning|SetWall%20Run%20IN (.ImpactNormal (Collision|BreakHitResult _outhit_2)))
        ;[0.00773 0 0.15 0.5] Checks fall speed
        (if (Utilities|FallSpeed)
          (WallRun|ApplyWRFLeft 1.0)
          (else
            (WallRun|ApplyWallRunVariable 1.0 false false false)))
        (else
          (goto _label))))))

(fn ApplyWRFRight
  (params (R%20-%20L :type Float%20%28double-precision%29))
  (WallRun|ApplyWallRunVariable 0.3 true true false)
  (Character|LaunchCharacter (Utilities|AttachPlayer(Wall)) false false)
  (Character|LaunchCharacter (Utilities|AlongWallVec R%20-%20L) true false))

(fn ApplyWRFLeft
  (params (R%20-%20L :type Float%20%28double-precision%29))
  (WallRun|ApplyWallRunVariable 0.3 true false true)
  (Character|LaunchCharacter (Utilities|AttachPlayer(Wall)) false false)
  (Character|LaunchCharacter (Utilities|AlongWallVec R%20-%20L) true false))

(fn ApplyWallRunVariable
  (params (Gravity%20Scale :type Float%20%28double-precision%29) (Wall%20Running :type Boolean) (Wall%20Running%20R :type Boolean) (Wall%20Running%20L :type Boolean))
  (Variables|/Script/Engine.CharacterMovementComponent|SetGravityScale (Variables|Character|GetCharacterMovement) Gravity%20Scale)
  (Variables|WallRunning|SetWall%20Running Wall%20Running)
  (Variables|WallRunning|SetWall%20Running%20R Wall%20Running%20R)
  (Variables|WallRunning|SetWall%20Running%20L Wall%20Running%20L))

(fn JumpfromWall
  (bind _wall_run_in (Variables|WallRunning|GetWall%20Run%20IN))
  (bind _returnvalue (* _wall_run_in 5e+02))
  (Character|LaunchCharacter (Math|Vector|MakeVector (.x _returnvalue) (.y _returnvalue) 5e+02) false true))

(fn CameraTilting
  (params (Rotation :type Float%20%28double-precision%29))
  (bind _returnvalue (Pawn|GetControlRotation :!class /Script/Engine.Pawn))
  (bind _returnvalue_2 (Pawn|GetController))
  (bind (_roll _pitch _yaw) (Math|Rotator|BreakRotator _returnvalue))
  (Utilities|IsValid _returnvalue_2
    (:Is%20Valid
      (Pawn|SetControlRotation _returnvalue_2 (Math|Interpolation|RInterpTo _returnvalue (Math|Rotator|MakeRotator Rotation _pitch _yaw) (Utilities|Time|GetWorldDeltaSeconds) 5.0)))))

(fn LoadPlayer
  (Input|AddMappingContext (PlayerController|LocalPlayerSubsystems|GetEnhancedInputLocalPlayerSubsystem (Game|GetPlayerController 0)) "/Game/Oscar_Coding/oscar_Inputs/IMC_PlayerControls.IMC_PlayerControls" 0 "(bIgnoreAllPressedKeysUntilRelease=True,bForceImmediately=False,bNotifyUserSettings=False)"))

(fn JumpBoostMath
  (params (Is%20Jump%20Boost :type Boolean) (InputPin :type Float%20%28double-precision%29))
  (bind _charactermovement (Variables|Character|GetCharacterMovement))
  (bind _charactermovement_2 (Variables|Character|GetCharacterMovement))
  (if (Variables|Character|GetHasLanded)
    (Variables|/Script/Engine.CharacterMovementComponent|SetJumpZVelocity (Variables|Character|GetCharacterMovement) 4.2e+02))
  (if (Variables|Character|GetIs%20Speed%20Boost)
    (Variables|Character|SetIs%20Jump%20Boost Is%20Jump%20Boost)
    (bind _output_get (Variables|Character|SetJump%20Boost InputPin))
    (Variables|/Script/Engine.CharacterMovementComponent|SetJumpZVelocity _charactermovement_2 (* _output_get (Variables|/Script/Engine.CharacterMovementComponent|GetJumpZVelocity _charactermovement_2)))
    (bind _output_get_2 (Variables|Character|SetSpeed%20Boost (Variables|Character|GetSpeed%20Boost)))
    (Variables|/Script/Engine.CharacterMovementComponent|SetMaxWalkSpeed (Variables|Character|GetCharacterMovement) (* _output_get_2 (Variables|Character|GetMax%20Sprint%20Speed)))
    (else
      (Variables|Character|SetIs%20Jump%20Boost Is%20Jump%20Boost)
      (bind _output_get_3 (Variables|Character|SetJump%20Boost InputPin))
      (Variables|/Script/Engine.CharacterMovementComponent|SetJumpZVelocity _charactermovement (* _output_get_3 (Variables|/Script/Engine.CharacterMovementComponent|GetJumpZVelocity _charactermovement))))))

(fn SpeedBoostMath
  (params (Is%20Speed%20Boost :type Boolean) (SpeedBoost :type Float%20%28double-precision%29))
  (if (Variables|Character|GetHasLanded)
    (Variables|/Script/Engine.CharacterMovementComponent|SetJumpZVelocity (Variables|Character|GetCharacterMovement) 4.2e+02))
  (if (Variables|Character|GetIs%20Jump%20Boost)
    (Variables|Character|SetIs%20Jump%20Boost true)
    (bind _output_get (Variables|Character|SetJump%20Boost (Variables|Character|GetJump%20Boost)))
    (Variables|/Script/Engine.CharacterMovementComponent|SetJumpZVelocity (Variables|Character|GetCharacterMovement) (* _output_get 4.2e+02))
    (bind _output_get_2 (Variables|Character|SetSpeed%20Boost (Variables|Character|GetSpeed%20Boost)))
    (bind _output_get_3 (Variables|/Script/Engine.CharacterMovementComponent|SetMaxWalkSpeed (Variables|Character|GetCharacterMovement) (* _output_get_2 (Variables|Character|GetMax%20Sprint%20Speed))))
    (Development|PrintString (Utilities|String|ToString(Float) _output_get_3))
    (else
      (Variables|Character|SetIs%20Speed%20Boost Is%20Speed%20Boost)
      (bind _output_get_4 (Variables|Character|SetSpeed%20Boost SpeedBoost))
      (Variables|/Script/Engine.CharacterMovementComponent|SetMaxWalkSpeed (Variables|Character|GetCharacterMovement) (* _output_get_4 (Variables|Character|GetMax%20Sprint%20Speed))))))

(fn PickItemSlot
  (params (PickedItem :type S%20Item%20Info%20Structure) (CurrSlot :type Integer))
  (if (.IsEmpty (Utilities|Struct|BreakS_ItemInfo (Utilities|Array|Get(acopy) (Variables|Default|GetItems) CurrSlot)))
    (Utilities|Array|SetArrayElem (Variables|Default|GetItems) CurrSlot PickedItem)
    (Class|BPIDelivery|SetIcon(Message) (Variables|Default|GetIWidget) CurrSlot (.ItemIcon (Utilities|Struct|BreakS_ItemInfo PickedItem)))))

(fn GetRefs
  (bind _returnvalue (Actor|GetActorOfClass "/Game/Oscar_Coding/oscar_Blueprints/Environment/BP_Zipline.BP_Zipline_C"))
  (Variables|ZiplineMechanic|SetZipline%20Actor _returnvalue)
  (bind _returnvalue_2 (UserInterface|CreateWidget "/Game/Oscar_Coding/oscar_Blueprints/UIElements/WBP_ItemBar.WBP_ItemBar_C" (Game|GetPlayerController 0)))
  (bind _output_get (Variables|Default|SetIWidget _returnvalue_2))
  (UserInterface|Viewport|AddtoViewport _output_get 0)
  (bind _returnvalue_3 (Actor|GetActorOfClass "/Game/Oscar_Coding/oscar_Blueprints/GameFrame/PS_Delivery.PS_Delivery_C"))
  (Variables|Default|SetPlayer%20State _returnvalue_3)
  (bind _returnvalue_4 (Actor|GetActorOfClass "/Game/Oscar_Coding/oscar_Blueprints/Environment/BP_Walls.BP_Walls_C"))
  (Variables|Default|SetWall%20Actor _returnvalue_4)
  (bind _asgame_i (Utilities|Casting|CastToGameI (Game|GetGameInstance)))
  (Variables|Default|SetAs%20Game%20I _asgame_i)
  (Variables|Default|SetItems (Variables|/Game/GameI.GameI_C|GetItems (Variables|Default|GetAs%20Game%20I))))

(fn DropItemfromSlot
  (bind _items (Variables|Default|GetItems))
  (bind _inventoryslot (Variables|Default|GetInventorySlot))
  (bind _inventoryslot_2 (Variables|Default|GetInventorySlot))
  (bind _empty (Variables|Default|GetEmpty))
  (bind _output (Utilities|Array|Get(acopy) _items _inventoryslot))
  (bind (_isempty _itemclass) (Utilities|Struct|BreakS_ItemInfo _output))
  (if (not _isempty)
    (Game|SpawnActorfromClass _itemclass (Math|Transform|MakeTransform (Transformation|GetWorldLocation (Variables|Default|GetDropItemRef)) "0, 0, 0" "1.000000,1.000000,1.000000") "Undefined" "MultiplyWithRoot" 0 0)
    (Utilities|Array|SetArrayElem (Variables|Default|GetItems) _inventoryslot_2 _empty)
    (Class|BPIDelivery|SetIcon(Message) (Variables|Default|GetIWidget) _inventoryslot_2 (.ItemIcon (Utilities|Struct|BreakS_ItemInfo _empty)))))

(fn ApplyStats
  (return ""))