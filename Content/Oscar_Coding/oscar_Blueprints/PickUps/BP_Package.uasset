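; Package pickup for the delivery game that the player collects by overlapping its sphere.
; BeginPlay caches the player, delivery PlayerState, drop-off and size-variant references.
; On overlap, it sends inventory space from its ApplyStats data to the PlayerState.
; If the current slot is empty, it also passes its item to the player, awards multiplied cash, updates the drop-off's package count, then destroys itself and forces garbage collection.
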(event OnComponentBeginOverlap(Sphere)
  (params (OverlappedComponent :type Primitive%20Component%20Object%20Reference) (OtherActor :type Actor%20Object%20Reference) (OtherComp :type Primitive%20Component%20Object%20Reference) (OtherBodyIndex :type Integer) (bFromSweep :type Boolean) (SweepResult :type Hit%20Result%20Structure%20%28by%20ref%29))
  (bind _player (Variables|Default|GetPlayer))
  ;[0.15 0.15 0.15 0.5] Apply Stats of pickup to player (checks if other actor has Apply Stats node)
  (if (== OtherActor (Variables|Default|GetPlayer))
    (bind _stats (Class|BPIDelivery|ApplyStats(Message) self))
    (Class|BPIDelivery|SetInventory(Message) (Variables|Default|GetPlayerState) (.invetoryspace _stats))
    (if (.IsEmpty (Utilities|Struct|BreakS_ItemInfo (Utilities|Array|Get(acopy) (Variables|/Game/Oscar_Coding/oscar_Blueprints/BP_Player.BP_Player_C|GetItems _player) (Variables|/Game/Oscar_Coding/oscar_Blueprints/BP_Player.BP_Player_C|GetInventorySlot _player))))
      (Class|BPIDelivery|ItemSelect(Message) (Variables|Default|GetPlayer) (Variables|Default|GetItemInfo) (Variables|/Game/Oscar_Coding/oscar_Blueprints/BP_Player.BP_Player_C|GetInventorySlot (Variables|Default|GetPlayer)))
      (bind _output_get (Variables|Default|SetCash (Math|Float|Truncate (* (.cashvalue _stats) (.cashmulti _stats)))))
      (Utilities|FlowControl|Sequence
        (:then_0
          (Class|BPIDelivery|AddCash(Message) (Game|GetPlayerState 0) _output_get))
        (:then_1
          (bind _output_get_2 (Variables|Default|SetPackagesToDeliver (+ 1 (Variables|Default|GetPackagesToDeliver))))
          (Class|BPIDelivery|CheckPackages(Message) (Variables|Default|GetDropOff) false _output_get_2))
        (:then_3
          (Actor|DestroyActor)
          (Utilities|Platform|CollectGarbage))))))

(event EventBeginPlay
  (CallFunction|GetRefs))

(fn ConstructionScript)

(fn GetRefs
  (bind _returnvalue (Actor|GetActorOfClass "/Game/Oscar_Coding/oscar_Blueprints/BP_Player.BP_Player_C"))
  (Variables|Default|SetPlayer _returnvalue)
  (bind _returnvalue_2 (Actor|GetActorOfClass "/Game/Oscar_Coding/oscar_Blueprints/GameFrame/PS_Delivery.PS_Delivery_C"))
  (Variables|Default|SetPlayerState _returnvalue_2)
  (bind _returnvalue_3 (Actor|GetActorOfClass "/Game/Oscar_Coding/oscar_Blueprints/PickUps/BP_Package_Large.BP_Package_Large_C"))
  (Variables|Default|SetLargeChild _returnvalue_3)
  (bind _returnvalue_4 (Actor|GetActorOfClass "/Game/Oscar_Coding/oscar_Blueprints/PickUps/BP_Package_Medium.BP_Package_Medium_C"))
  (Variables|Default|SetMediumChild _returnvalue_4)
  (bind _returnvalue_5 (Actor|GetActorOfClass "/Game/Oscar_Coding/oscar_Blueprints/PickUps/BP_Package_Small.BP_Package_Small_C"))
  (Variables|Default|SetSmallChild _returnvalue_5)
  (bind _returnvalue_6 (Actor|GetActorOfClass "/Game/Oscar_Coding/oscar_Blueprints/Environment/BP_DropOff.BP_DropOff_C"))
  (Variables|Default|SetDropOff _returnvalue_6))

(fn ApplyStats
  (return (Variables|Default|GetStats)))