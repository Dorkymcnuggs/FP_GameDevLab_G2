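; BP_JumpBoost is a pickup that gives the player a jump boost item.
; On sphere overlap with BP_Player, it passes its inventory space value to PS_Delivery, then, if the selected slot is empty, gives the item, plays a pop and destroys itself.
; ActivateConsume sends the boost from its Stats, read through the ApplyStats message, to the player with a neutral speed boost.
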(event OnComponentBeginOverlap(Sphere)
  (params (OverlappedComponent :type Primitive%20Component%20Object%20Reference) (OtherActor :type Actor%20Object%20Reference) (OtherComp :type Primitive%20Component%20Object%20Reference) (OtherBodyIndex :type Integer) (bFromSweep :type Boolean) (SweepResult :type Hit%20Result%20Structure%20%28by%20ref%29))
  (bind _player (Variables|Default|GetPlayer))
  ;[0.15 0.15 0.15 0.5] Apply Stats of pickup to player (checks if other actor has Apply Stats node)
  (if (== OtherActor (Variables|Default|GetPlayer))
    (bind _stats (Class|BPIDelivery|ApplyStats(Message) self))
    (Class|BPIDelivery|SetInventory(Message) (Variables|Default|GetPlayerState) (.invetoryspace _stats))
    (if (.IsEmpty (Utilities|Struct|BreakS_ItemInfo (Utilities|Array|Get(acopy) (Variables|/Game/Oscar_Coding/oscar_Blueprints/BP_Player.BP_Player_C|GetItems _player) (Variables|/Game/Oscar_Coding/oscar_Blueprints/BP_Player.BP_Player_C|GetInventorySlot _player))))
      (Utilities|FlowControl|Sequence
        (:then_0
          (Class|BPIDelivery|ItemSelect(Message) (Variables|Default|GetPlayer) (Variables|Default|GetItemInfo) (Variables|/Game/Oscar_Coding/oscar_Blueprints/BP_Player.BP_Player_C|GetInventorySlot (Variables|Default|GetPlayer)))
          (Audio|PlaySound2D "/Game/sound/pop.pop" 1.0 1.4 0.0 0 0))
        (:then_1
          (Actor|DestroyActor))))))

(event EventBeginPlay
  (bind _returnvalue (Actor|GetActorOfClass "/Game/Oscar_Coding/oscar_Blueprints/BP_Player.BP_Player_C"))
  (Variables|Default|SetPlayer _returnvalue)
  (bind _returnvalue_2 (Actor|GetActorOfClass "/Game/Oscar_Coding/oscar_Blueprints/GameFrame/PS_Delivery.PS_Delivery_C"))
  (Variables|Default|SetPlayerState _returnvalue_2))

(event EventActivateConsume
  ;[0.15 0.15 0.15 0.5] Apply Stats of pickup to player (checks if other actor has Apply Stats node)
  (bind _stats (Class|BPIDelivery|ApplyStats(Message) self))
  (bind _output_get (Variables|Default|SetIsJumpBoost (.isjumpboost _stats)))
  (bind _output_get_2 (Variables|Default|SetJump%20Boost (.jumpboost _stats)))
  (Class|BPIDelivery|ApplyBoosts(Message) (Variables|Default|GetPlayer) _output_get _output_get_2 false 1.0))

(fn ConstructionScript)

(fn ApplyStats
  (return (Variables|Default|GetStats)))