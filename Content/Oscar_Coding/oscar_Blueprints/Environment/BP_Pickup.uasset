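; BP_Pickup is a cardboard box pickup that players collect by walking into it to earn points.
; On overlap it casts to BP_Player and checks that the player's remaining Inventory is above zero.
; If so, helper functions add the pickup's Value to Score and decrement Inventory, then the actor destroys itself.
; Debug prints report the collection and score, or that the player is carrying too much.
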(event EventBeginPlay)

(event Collision|EventActorBeginOverlap
  (params (OtherActor :type Actor%20Object%20Reference))
  (bind _asbp_player (Utilities|Casting|CastToBP_Player OtherActor))
  (if (== OtherActor _asbp_player)
    (if (> (Variables|/Game/Oscar_Coding/oscar_Blueprints/BP_Player.BP_Player_C|GetInventory _asbp_player) 0)
      (bind _output_get (|PointAllocation _asbp_player))
      (|InventorySpace _asbp_player)
      (Actor|DestroyActor)
      (Development|PrintString "Noice A Cardboard box")
      (Development|PrintString (Utilities|String|ToString(Float) _output_get) true true "(R=0.000000,G=0.660000,B=1.000000,A=1.000000)" 4.0)
      (else
        (Development|PrintString "Dam I'm already carrying too much")))))

(fn ConstructionScript)