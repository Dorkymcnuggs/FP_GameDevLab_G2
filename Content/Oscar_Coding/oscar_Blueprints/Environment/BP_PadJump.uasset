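; BP_PadJump is a jump pad that launches the player character and plays a boing sound.
; On BeginPlay it caches BP_Player, and any Box overlap launches that player without checking which actor entered.
; Launch overrides velocity with the Arrow's forward vector scaled by LaunchVelocityZ, plus a fixed upward boost.
; The HoriVerti flag is checked, but both branches behave identically.
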(event OnComponentBeginOverlap(Box)
  (params (OverlappedComponent :type Primitive%20Component%20Object%20Reference) (OtherActor :type Actor%20Object%20Reference) (OtherComp :type Primitive%20Component%20Object%20Reference) (OtherBodyIndex :type Integer) (bFromSweep :type Boolean) (SweepResult :type Hit%20Result%20Structure%20%28by%20ref%29))
  (bind _player (Variables|Default|GetPlayer)
    (:then
      (if (Variables|Default|GetHori/Verti)
        (Audio|PlaySound2D "/Game/sound/boing.boing" 1.0 1.0 0.0 0 0)
        (CallFunction|Launch _player)
        (else
          (Audio|PlaySound2D "/Game/sound/boing.boing" 1.0 1.0 0.0 0 0)
          (CallFunction|Launch _player))))
    (:else)))

(event EventBeginPlay
  (bind _returnvalue (Actor|GetActorOfClass "/Game/Oscar_Coding/oscar_Blueprints/BP_Player.BP_Player_C"))
  (Variables|Default|SetPlayer _returnvalue))

(event Collision|EventActorBeginOverlap
  (params (OtherActor :type Actor%20Object%20Reference)))

(event EventTick
  (params (DeltaSeconds :type Float%20%28single-precision%29)))

(fn ConstructionScript)

(fn Launch
  (params (self2 :type Character%20Object%20Reference))
  (Character|LaunchCharacter self2 (+ (* (Math|Vector|GetForwardVector (Variables|Default|GetArrow)) (Variables|Default|GetLaunch%20Velocity%20Z)) "0.000000,0.000000,500.000000") true true))