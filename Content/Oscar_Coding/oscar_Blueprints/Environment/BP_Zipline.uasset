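; Zipline actor that carries the player along a spline when its collision is overlapped.
; On overlap it flags the cached BP_Player and finds the nearest spline distance, then a timeline lerps the player to the spline's end, 100 units below the line.
; Leaving the collision clears zipline state, switches movement to falling and sends neutral boosts.
; An ApplyBoosts event also scales the player's jump velocity and walk speed.
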(event OnComponentBeginOverlap(ZiplineCollision)
  (params (OverlappedComponent :type Primitive%20Component%20Object%20Reference) (OtherActor :type Actor%20Object%20Reference) (OtherComp :type Primitive%20Component%20Object%20Reference) (OtherBodyIndex :type Integer) (bFromSweep :type Boolean) (SweepResult :type Hit%20Result%20Structure%20%28by%20ref%29))
  (bind _as_bp_player (Variables|Default|GetAs%20BP%20Player))
  (bind _spline (Variables|Default|GetSpline))
  (bind _returnvalue (Spline|GetSplineLength _spline))
  (Variables|/Game/Oscar_Coding/oscar_Blueprints/BP_Player.BP_Player_C|SetNearZipline? _as_bp_player true)
  (Variables|/Game/Oscar_Coding/oscar_Blueprints/BP_Player.BP_Player_C|SetZipline%20Actor _as_bp_player self)
  (bind _output_get (Variables|Default|SetCurStart (Class|SplineComponent|GetDistanceAlongSplineatLocation (Variables|Default|GetSpline) (Transformation|GetActorLocation _as_bp_player) "World")))
  (bind _down_zipline (Timeline|Timeline PlayFromStart)
    (:Update
      (|MoveAlongZipline _down_zipline _returnvalue (Variables|Default|GetCurStart)))))

(event OnComponentEndOverlap(ZiplineCollision)
  (params (OverlappedComponent :type Primitive%20Component%20Object%20Reference) (OtherActor :type Actor%20Object%20Reference) (OtherComp :type Primitive%20Component%20Object%20Reference) (OtherBodyIndex :type Integer))
  (bind _as_bp_player (Variables|Default|GetAs%20BP%20Player))
  (Variables|/Game/Oscar_Coding/oscar_Blueprints/BP_Player.BP_Player_C|SetWas%20Ziplining _as_bp_player true)
  (Variables|/Game/Oscar_Coding/oscar_Blueprints/BP_Player.BP_Player_C|SetNearZipline? _as_bp_player false)
  (Variables|/Game/Oscar_Coding/oscar_Blueprints/BP_Player.BP_Player_C|SetZipline%20Actor _as_bp_player 0)
  (Variables|/Game/Oscar_Coding/oscar_Blueprints/BP_Player.BP_Player_C|SetIsZiplining _as_bp_player false)
  (Pawn|Components|CharacterMovement|SetMovementMode (Variables|/Script/Engine.Character|GetCharacterMovement _as_bp_player) "MOVE_Falling" 0)
  (Class|BPIDelivery|ApplyBoosts(Message) self false 1.0 false 1.0))

(event EventBeginPlay
  (bind _returnvalue (Actor|GetActorOfClass "/Game/Oscar_Coding/oscar_Blueprints/BP_Player.BP_Player_C"))
  (Variables|Default|SetAs%20BP%20Player _returnvalue))

(event Collision|EventActorBeginOverlap
  (params (OtherActor :type Actor%20Object%20Reference)))

(event EventTick
  (params (DeltaSeconds :type Float%20%28single-precision%29)))

(event EventApplyBoosts
  (params (IsJumpBoost :type Boolean) (JumpBoost :type Float%20%28double-precision%29) (IsSpeedBoost :type Boolean) (SpeedBoost :type Float%20%28double-precision%29))
  (Utilities|FlowControl|Sequence
    (:then_0
      (if IsJumpBoost
        (CallFunction|JumpBoostMath IsJumpBoost JumpBoost)))
    (:then_1
      (if IsSpeedBoost
        (CallFunction|SpeedBoostMath IsSpeedBoost SpeedBoost)))))

(fn ConstructionScript)

(fn JumpBoostCheck
  (params (self2 :type Character%20Movement%20Component%20Object%20Reference))
  (Variables|/Script/Engine.CharacterMovementComponent|SetJumpZVelocity self2 (* 4.2e+02 (Variables|Default|GetJump%20Boost)))
  (return (Variables|Default|GetIs%20Jump%20Boost)))

(fn SpeedBoostCheck
  (bind _as_bp_player (Variables|Default|GetAs%20BP%20Player))
  (Variables|/Script/Engine.CharacterMovementComponent|SetMaxWalkSpeed (Variables|/Script/Engine.Character|GetCharacterMovement _as_bp_player) (* (Variables|/Game/Oscar_Coding/oscar_Blueprints/BP_Player.BP_Player_C|GetMax%20Sprint%20Speed _as_bp_player) (Variables|Default|GetSpeed%20Boost)))
  (return (Variables|Default|GetIs%20Speed%20Boost)))

(fn SpeedBoostMath
  (params (IsSpeedBoost :type Boolean) (SpeedBoost :type Float%20%28double-precision%29))
  (bind _as_bp_player (Variables|Default|GetAs%20BP%20Player))
  (bind _as_bp_player_2 (Variables|Default|GetAs%20BP%20Player))
  (bind _charactermovement (Variables|/Script/Engine.Character|GetCharacterMovement _as_bp_player_2))
  (if (Variables|Default|GetIs%20Jump%20Boost)
    (Variables|Default|SetIs%20Jump%20Boost true)
    (bind _output_get (Variables|Default|SetJump%20Boost (Variables|Default|GetJump%20Boost)))
    (Variables|/Script/Engine.CharacterMovementComponent|SetJumpZVelocity _charactermovement (* _output_get (Variables|/Script/Engine.CharacterMovementComponent|GetJumpZVelocity _charactermovement)))
    (bind _output_get_2 (Variables|Default|SetSpeed%20Boost (Variables|Default|GetSpeed%20Boost)))
    (Variables|/Script/Engine.CharacterMovementComponent|SetMaxWalkSpeed (Variables|/Script/Engine.Character|GetCharacterMovement _as_bp_player) (* _output_get_2 (Variables|/Game/Oscar_Coding/oscar_Blueprints/BP_Player.BP_Player_C|GetMax%20Sprint%20Speed _as_bp_player)))
    (else
      (Variables|Default|SetIs%20Speed%20Boost IsSpeedBoost)
      (bind _output_get_3 (Variables|Default|SetSpeed%20Boost SpeedBoost))
      (Variables|/Script/Engine.CharacterMovementComponent|SetMaxWalkSpeed (Variables|/Script/Engine.Character|GetCharacterMovement (Variables|Default|GetAs%20BP%20Player)) (* _output_get_3 0.0)))))

(fn JumpBoostMath
  (params (IsJumpBoost :type Boolean) (JumpBoost :type Float%20%28double-precision%29))
  (bind _as_bp_player (Variables|Default|GetAs%20BP%20Player))
  (bind _as_bp_player_2 (Variables|Default|GetAs%20BP%20Player))
  (bind _as_bp_player_3 (Variables|Default|GetAs%20BP%20Player))
  (bind _charactermovement (Variables|/Script/Engine.Character|GetCharacterMovement _as_bp_player_2))
  (bind _charactermovement_2 (Variables|/Script/Engine.Character|GetCharacterMovement _as_bp_player_3))
  (if (Variables|Default|GetIs%20Speed%20Boost)
    (Variables|Default|SetIs%20Jump%20Boost IsJumpBoost)
    (bind _output_get (Variables|Default|SetJump%20Boost JumpBoost))
    (Variables|/Script/Engine.CharacterMovementComponent|SetJumpZVelocity _charactermovement_2 (* _output_get (Variables|/Script/Engine.CharacterMovementComponent|GetJumpZVelocity _charactermovement_2)))
    (Variables|Default|SetIs%20Speed%20Boost (Variables|Default|GetIs%20Speed%20Boost))
    (bind _output_get_2 (Variables|Default|SetSpeed%20Boost (Variables|Default|GetSpeed%20Boost)))
    (Variables|/Script/Engine.CharacterMovementComponent|SetMaxWalkSpeed (Variables|/Script/Engine.Character|GetCharacterMovement _as_bp_player) (* _output_get_2 (Variables|/Game/Oscar_Coding/oscar_Blueprints/BP_Player.BP_Player_C|GetMax%20Sprint%20Speed _as_bp_player)))
    (else
      (Variables|Default|SetIs%20Jump%20Boost IsJumpBoost)
      (bind _output_get_3 (Variables|Default|SetJump%20Boost JumpBoost))
      (Variables|/Script/Engine.CharacterMovementComponent|SetJumpZVelocity _charactermovement (* _output_get_3 (Variables|/Script/Engine.CharacterMovementComponent|GetJumpZVelocity _charactermovement))))))

(fn ApplyStats
  (return ""))