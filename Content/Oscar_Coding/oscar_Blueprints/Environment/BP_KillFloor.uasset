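; BP_KillFloor is a kill volume that costs the player a life on overlap and respawns them.
; Its box overlap sends a life decrement to the player state, then triggers a death sequence if lives remain, or only garbage collection at zero.
; The death sequence teleports the pawn to the respawn location of the BP_RespawnActor cached at BeginPlay and matches the controller's rotation.
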(event OnComponentBeginOverlap(Box)
  (params (OverlappedComponent :type Primitive%20Component%20Object%20Reference) (OtherActor :type Actor%20Object%20Reference) (OtherComp :type Primitive%20Component%20Object%20Reference) (OtherBodyIndex :type Integer) (bFromSweep :type Boolean) (SweepResult :type Hit%20Result%20Structure%20%28by%20ref%29))
  (if (== OtherActor (Game|Player|GetPlayerPawn 0))
    (Class|BPIDelivery|AddLives(Message) (Game|GetPlayerState 0) -1)
    (if (== (Variables|/Game/Oscar_Coding/oscar_Blueprints/GameFrame/PS_Delivery.PS_Delivery_C|GetPlayer%20Lives (Variables|Default|GetPlayerState)) 0)
      (Utilities|Platform|CollectGarbage)
      (else
        (Class|BPIDelivery|DeathSequence(Message) self)))))

(event EventBeginPlay
  (bind _returnvalue (Actor|GetActorOfClass "/Script/Engine.PlayerStart"))
  (Variables|Default|SetPlayStart _returnvalue)
  (bind _returnvalue_2 (Actor|GetActorOfClass "/Game/Oscar_Coding/oscar_Blueprints/BP_Player.BP_Player_C"))
  (Variables|Default|SetPlayer _returnvalue_2)
  (bind _returnvalue_3 (Actor|GetActorOfClass "/Game/Oscar_Coding/oscar_Blueprints/GameFrame/PS_Delivery.PS_Delivery_C"))
  (Variables|Default|SetPlayerState _returnvalue_3)
  (bind _returnvalue_4 (Actor|GetActorOfClass "/Game/Oscar_Coding/oscar_Blueprints/Environment/BP_RespawnActor.BP_RespawnActor_C"))
  (Variables|Default|Setrespawn%20point _returnvalue_4))

(event EventDeathSequence
  (bind _respawn_point (Variables|Default|Getrespawn%20point))
  (bind _respawnloc (Variables|/Game/Oscar_Coding/oscar_Blueprints/Environment/BP_RespawnActor.BP_RespawnActor_C|GetRespawnLOC _respawn_point))
  (Transformation|SetActorTransform (Game|Player|GetPlayerPawn 0) (Math|Transform|MakeTransform (.location _respawnloc) (.rotation _respawnloc) "1.000000,1.000000,1.000000") false true)
  (Transformation|SetActorRotation (Game|GetPlayerController 0) (.rotation _respawnloc) true))

(fn ConstructionScript)

(fn ApplyStats
  (return ""))