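; Drop-off zone where the player hands in packages to end the day and move on to the Shop level.
; On overlap with BP_Player, it clears package-type items from the inventory, updates their slot icons and adds them to a running count.
; A CheckPackages message compares that count to TotalPackages, either flagging delivery complete or printing a prompt to get more.
; Once complete, it removes the HUD and inventory widgets, increments Days and opens Shop.
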(event OnComponentBeginOverlap(Box)
  (params (OverlappedComponent :type Primitive%20Component%20Object%20Reference) (OtherActor :type Actor%20Object%20Reference) (OtherComp :type Primitive%20Component%20Object%20Reference) (OtherBodyIndex :type Integer) (bFromSweep :type Boolean) (SweepResult :type Hit%20Result%20Structure%20%28by%20ref%29))
  (if (== OtherActor (Variables|Default|GetBPPlayer))
    (CallFunction|CustomEvent self)
    (if (Variables|Default|GetDeliveredPackages)
      (Variables|Default|SetItemInfo (Utilities|Struct|MakeS_ItemInfo "None" 0 true 0 "NewEnumerator3" 0))
      (Widget|RemovefromParent (Variables|Default|GetPlayerHUD))
      (Widget|RemovefromParent (Variables|Default|GetPlayerInventory))
      (Variables|Default|SetDays (+ (Variables|Default|GetDays) 1))
      (Game|OpenLevel(byName) "Shop")
      (Utilities|Platform|CollectGarbage))))

(event Custom|CustomEvent
  (bind _bpplayer (Variables|Default|GetBPPlayer))
  (for (_array_element _array_index) (Variables|/Game/Oscar_Coding/oscar_Blueprints/BP_Player.BP_Player_C|GetItems (Variables|Default|GetBPPlayer))
    (Variables|Default|SetArray%20Index _array_index)
    (if (Utilities|Enum|Equal(Enum) (.ItemType (Utilities|Struct|BreakS_ItemInfo _array_element)) "NewEnumerator0")
      (Variables|Default|SetPackagesInventory (+ (Variables|Default|GetPackagesInventory) 1))
      (Utilities|Array|SetArrayElem (Variables|/Game/Oscar_Coding/oscar_Blueprints/BP_Player.BP_Player_C|GetItems _bpplayer) (Variables|Default|GetArray%20Index) (Variables|/Game/Oscar_Coding/oscar_Blueprints/BP_Player.BP_Player_C|GetEmpty _bpplayer))
      (Class|BPIDelivery|SetIcon(Message) (Variables|/Game/Oscar_Coding/oscar_Blueprints/BP_Player.BP_Player_C|GetIWidget (Variables|Default|GetBPPlayer)) (Variables|Default|GetArray%20Index) "/Game/Oscar_Coding/oscar_Materials/T_EmptySlotCon.T_EmptySlotCon")))
  (Class|BPIDelivery|CheckPackages(Message) self false (Variables|Default|GetPackagesInventory)))

(event EventBeginPlay
  (CallFunction|GetRefs))

(event Collision|EventActorBeginOverlap
  (params (OtherActor :type Actor%20Object%20Reference)))

(event EventTick
  (params (DeltaSeconds :type Float%20%28single-precision%29)))

(event EventCheckPackages
  (params (HasDeliveredAll :type Boolean) (PackagesToDeliver :type Integer))
  (if (not HasDeliveredAll)
    (if (<= (- (Variables|Default|GetTotalPackages) PackagesToDeliver) 0)
      (Variables|Default|SetDeliveredPackages true)
      (else
        (Development|PrintString "Go get more packages")))))

(fn ConstructionScript)

(fn GetRefs
  (bind _returnvalue (Actor|GetActorOfClass "/Game/Oscar_Coding/oscar_Blueprints/BP_Player.BP_Player_C"))
  (Variables|Default|SetBPPlayer _returnvalue)
  (bind _returnvalue_2 (UserInterface|CreateWidget "/Game/Oscar_Coding/oscar_Blueprints/UIElements/WBP_PlayerHUD.WBP_PlayerHUD_C" (Game|GetPlayerController 0)))
  (Variables|Default|SetPlayerHUD _returnvalue_2)
  (bind _returnvalue_3 (UserInterface|CreateWidget "/Game/ArthurProtypecrap/ShopUI.ShopUI_C" (Game|GetPlayerController 0)))
  (Variables|Default|SetShopUi _returnvalue_3)
  (bind _returnvalue_4 (Actor|GetActorOfClass "/Game/Oscar_Coding/oscar_Blueprints/GameFrame/PS_Delivery.PS_Delivery_C"))
  (Variables|Default|SetPlayer%20State _returnvalue_4)
  (bind _returnvalue_5 (Actor|GetActorOfClass "/Game/Oscar_Coding/oscar_Blueprints/PickUps/BP_Package.BP_Package_C"))
  (Variables|Default|SetPackage _returnvalue_5))

(fn ApplyStats
  (return ""))